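; CollisionPawnOverlap is a Blueprint that visualizes and reports overlaps on its Sphere component, apparently for debugging collision.
; When another actor begins overlapping the Sphere, it draws a short-lived black debug line from the sphere's location to that actor.
; It then prints its own display name, the word "overlaps" and the other actor's name as separate messages.
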(event `self.Sphere.OnComponentBeginOverlap`
  (params (OverlappedComponent :type "PrimitiveComponent Object Reference") (OtherActor :type "Actor Object Reference") (OtherComp :type "PrimitiveComponent Object Reference") (OtherBodyIndex :type Integer) (bFromSweep :type Boolean) (SweepResult :type "HitResult Structure (by ref)"))
  (`|ExecutionSequence`
    (:`then_0`
      (`KismetSystemLibrary.DrawDebugLine` (`SceneComponent.K2_GetComponentLocation` (`self.Sphere`)) (`self.K2_GetActorLocation` OtherActor) (struct :`A` 1.0) 1.0 3.0))
    (:`then_1`
      (`KismetSystemLibrary.PrintString` (`KismetSystemLibrary.GetDisplayName` self))
      (`KismetSystemLibrary.PrintString` "overlaps")
      (`KismetSystemLibrary.PrintString` (`KismetSystemLibrary.GetDisplayName` OtherActor)))))

(fn `UserConstructionScript`)