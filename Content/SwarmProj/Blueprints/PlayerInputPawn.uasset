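; PlayerInputPawn is a pawn that the player takes control of by entering its collision sphere, and leaves by pressing F.
; Overlap begin enables input, hides the current player pawn and immediately possesses this pawn, despite its "Press F" debug message.
; F re-possesses and unhides the original pawn cached on BeginPlay, while overlap end disables input.
; The overlap events do not check which actor triggered them.
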(event `Key|F` :paused true
  (params (Key :type "Key Structure"))
  (:`Pressed`
    (`|ExecutionSequence`
      (:`then_0`
        (`KismetSystemLibrary.PrintString` "F pressed"))
      (:`then_1`
        (`Controller.Possess` (`GameplayStatics.GetPlayerController` 0) (stale `self.ReceiveBeginPlay` _output_get)))
      (:`then_2`
        (`self.SetActorHiddenInGame` (stale `self.ReceiveBeginPlay` _output_get) false)))))

(event `self.ReceiveBeginPlay`
  (bind _output_get (set `self.DefaultPlayerPawn` (`GameplayStatics.GetPlayerPawn` 0))))

(event `self.Spherecollision.OnComponentBeginOverlap`
  (params (OverlappedComponent :type "PrimitiveComponent Object Reference") (OtherActor :type "Actor Object Reference") (OtherComp :type "PrimitiveComponent Object Reference") (OtherBodyIndex :type Integer) (bFromSweep :type Boolean) (SweepResult :type "HitResult Structure (by ref)"))
  (bind _returnvalue (`GameplayStatics.GetPlayerController` 0))
  (`|ExecutionSequence`
    (:`then_0`
      (`self.EnableInput` _returnvalue))
    (:`then_1`
      (`KismetSystemLibrary.PrintString` "object controllable. Press F"))
    (:`then_2`
      (`self.SetActorHiddenInGame` (`GameplayStatics.GetPlayerPawn` 0) true))
    (:`then_3`
      (`Controller.Possess` _returnvalue self))))

(event `self.Spherecollision.OnComponentEndOverlap`
  (params (OverlappedComponent :type "PrimitiveComponent Object Reference") (OtherActor :type "Actor Object Reference") (OtherComp :type "PrimitiveComponent Object Reference") (OtherBodyIndex :type Integer))
  (`|ExecutionSequence`
    (:`then_0`
      (`self.DisableInput` (`GameplayStatics.GetPlayerController` 0)))
    (:`then_1`
      (`KismetSystemLibrary.PrintString` "object no longer controllable"))))

(fn `UserConstructionScript`)