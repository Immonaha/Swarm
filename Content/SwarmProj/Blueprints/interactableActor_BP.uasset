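; An interactable actor that a player can trigger with the F key while something overlaps its box collision, with a debug "Hello" print as the only action so far.
; Begin overlap enables input from player controller 0, prints a prompt and swaps the cube's material as a highlight.
; End overlap disables input, prints a notice and sets the other material.
; Neither overlap event checks which actor caused it.
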(event `Key|F` :paused true
  (params (Key :type "Key Structure"))
  (:`Pressed`
    (`KismetSystemLibrary.PrintString` "Hello")))

(event `self.BoxCollision.OnComponentBeginOverlap`
  (params (OverlappedComponent :type "PrimitiveComponent Object Reference") (OtherActor :type "Actor Object Reference") (OtherComp :type "PrimitiveComponent Object Reference") (OtherBodyIndex :type Integer) (bFromSweep :type Boolean) (SweepResult :type "HitResult Structure (by ref)"))
  (`|ExecutionSequence`
    (:`then_0`
      (`self.EnableInput` (`GameplayStatics.GetPlayerController` 0)))
    (:`then_1`
      (`KismetSystemLibrary.PrintString` "object controllable. Press F"))
    (:`then_2`
      (`PrimitiveComponent.SetMaterial` (`self.Cube`) 0 "/Game/SwarmProj/Mats/CryingGlassMat2.CryingGlassMat2"))))

(event `self.BoxCollision.OnComponentEndOverlap`
  (params (OverlappedComponent :type "PrimitiveComponent Object Reference") (OtherActor :type "Actor Object Reference") (OtherComp :type "PrimitiveComponent Object Reference") (OtherBodyIndex :type Integer))
  (`|ExecutionSequence`
    (:`then_0`
      (`self.DisableInput` (`GameplayStatics.GetPlayerController` 0)))
    (:`then_1`
      (`KismetSystemLibrary.PrintString` "object no longer controllable"))
    (:`then_2`
      (`PrimitiveComponent.SetMaterial` (`self.Cube`) 0 "/Game/SwarmProj/Mats/CryingGlassMat.CryingGlassMat"))))

(fn `UserConstructionScript`)